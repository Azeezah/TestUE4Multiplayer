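; CustomPlayerController is a player controller that makes the controlled SpherePawnBP move up when Space Bar is pressed.
; The key handler calls MoveUp on the pawn directly, then calls a ServerMoveUp event that repeats the cast and call, apparently to mirror the move on the server.
; Print strings trace BeginPlay, the key press and the server event.
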(event Custom|ServerMoveUp
  (Development|PrintString "Server move up")
  (bind _assphere_pawn_bp (Utilities|Casting|CastToSpherePawnBP (Pawn|GetControlledPawn)))
  (Default|MoveUp _assphere_pawn_bp))

(event EventBeginPlay
  (Development|PrintString "in controller"))

(event EventTick
  (params (DeltaSeconds :type Float%20%28single-precision%29)))

(event Input|KeyboardEvents|SpaceBar
  (params (Key :type Key%20Structure :default "None"))
  (:Pressed
    (Development|PrintString "Hit spacebar")
    (bind _assphere_pawn_bp (Utilities|Casting|CastToSpherePawnBP (Pawn|GetControlledPawn)))
    (Default|MoveUp _assphere_pawn_bp)
    (CallFunction|ServerMoveUp)))

(fn ConstructionScript)